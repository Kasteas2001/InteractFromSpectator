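; Base interactive object actor for the SuperSpectator project, configured through variables that set its look and label.
; The construction script calls UpdateInteractive, which applies the selected entry from a material map to the first slot of every static mesh component.
; It also writes the name to a text component and sets visibility and color on all point lights.
; The event graph has no runtime logic.
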(event `self.ReceiveBeginPlay`)

(fn `UpdateInteractive`
  (bind (_value _returnvalue) (`BlueprintMapLibrary.Map_Find` (`self.Material`) (`self.SelectedMaterial`)))
  (`|ExecutionSequence`
    (:`then_0`
      (if _returnvalue
        (for _array_element (`self.K2_GetComponentsByClass` "/Script/Engine.StaticMeshComponent")
          (`PrimitiveComponent.SetMaterial` _array_element 0 _value))))
    (:`then_1`
      (`TextRenderComponent.K2_SetText` (`self.Text_Name`) (`self.Name`)))
    (:`then_2`
      (for _array_element_2 (`self.K2_GetComponentsByClass` "/Script/Engine.PointLightComponent")
        (`SceneComponent.SetVisibility` _array_element_2 (`self.Light`) false)
        (`LightComponent.SetLightColor` _array_element_2 (`self.Light Color`) true)))))

(fn `UserConstructionScript`
  (`self.UpdateInteractive`))