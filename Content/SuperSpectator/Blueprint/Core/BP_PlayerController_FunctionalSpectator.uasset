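; Player controller that lets the player toggle between their third-person character and a spectator pawn with Tab.
; It caches the player's BP_ThirdPersonCharacter_Child on BeginPlay and tracks spectator state with a flag.
; Switching to spectator possesses a BP_Spectator spawned at the character's location and rotation, or an existing valid one.
; Switching back destroys the spectator and repossesses the character.
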(event `self.ReceiveBeginPlay`
  (`|ExecutionSequence`
    (:`then_0`
      (bind _asbp_third_person_character_child (cast `/Game/SuperSpectator/Blueprint/Pawn/BP_ThirdPersonCharacter_Child` (`GameplayStatics.GetPlayerCharacter` 0)))
      (set `self.CharacterRef` _asbp_third_person_character_child))
    (:`then_1`
      (set `self.IsPlayerSpectator?` false))))

(event `Key|Tab`
  (params (Key :type "Key Structure"))
  (:`Pressed`
    (`self.SwitchPawn`)))

(event `self.ReceiveTick`
  (params (DeltaSeconds :type "Float (single-precision)")))

(fn `CurrentPawnSpectator?`)

(fn `SwitchPawn`
  (bind _characterref (`self.CharacterRef`))
  (if (`self.IsPlayerSpectator?`)
    (bind _spectatorpawnref (`self.SpectatorPawnRef`)
      (:`then`
        (`self.K2_DestroyActor` _spectatorpawnref))
      (:`else`
        _))
    (bind _characterref_2 (`self.CharacterRef`)
      (:`then`
        (`self.Possess` _characterref_2)
        (set `self.IsPlayerSpectator?` false))
      (:`else`))
    (else
      (bind _spectatorpawnref_2 (`self.SpectatorPawnRef`)
        (:`then`
          (`self.Possess` _spectatorpawnref_2))
        (:`else`
          (bind _returnvalue (`|SpawnActorFromClass` "/Game/SuperSpectator/Blueprint/Pawn/BP_Spectator.BP_Spectator_C" (`KismetMathLibrary.MakeTransform` (`self.K2_GetActorLocation` _characterref) (`self.K2_GetActorRotation` _characterref)) "Undefined" "MultiplyWithRoot" null (`self.CharacterRef`)))
          (`self.Possess` _returnvalue)
          (set `self.SpectatorPawnRef` _returnvalue)))
      (set `self.IsPlayerSpectator?` true))))

(fn `UserConstructionScript`)